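; Ranged enemy Blueprint that spawns a pistol on BeginPlay, attaches it to its hand socket and fires it at the AI controller's attack target.
; Attack plays a fire montage whose notify runs a debug-drawn visibility trace from pistol to target.
; Any blocking hit damages the target through both an interface message and ApplyDamage, without checking which actor was hit.
; Montage completion or interruption signals attack end.
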(event `self.ReceiveBeginPlay`
  (`parent.ReceiveBeginPlay`)
  (`/Game/Enemies/AI/BPI_EnemyAI_Base.EquipWeapon`))

(event `/Game/Enemies/AI/BPI_EnemyAI_Base.Attack`
  (bind _notifyname (`|PlayMontage` (`self.Mesh`) "/Game/Sword_Animation/Animations/Montage_FireBullet.Montage_FireBullet")
    (:`OnCompleted`
      (`self.OnAttackEnd` :!label _label))
    (:`OnInterrupted`
      (goto _label))
    (:`OnNotifyBegin`
      (switch `name` _notifyname
        (:`Fire`
          (bind _asaic_enemy_base (cast `/Game/Enemies/AI/AIC_Enemy_Base` (`AIBlueprintHelperLibrary.GetAIController` self)))
          (bind _attacktarget (`/Game/Enemies/AI/AIC_Enemy_Base.AttackTarget` _asaic_enemy_base)
            (:`then`
              (bind (_outhit _returnvalue) (`KismetSystemLibrary.LineTraceSingle` :`Start` (`self.K2_GetActorLocation` (`self.PistolActor`)) :`End` (`self.K2_GetActorLocation` _attacktarget) :`TraceChannel` "TraceTypeQuery1" :`DrawDebugType` "ForDuration"))
              (if _returnvalue
                (message `/Game/DamageSystem/BPI_Damagble.TakeDamage` _attacktarget (make `/Game/DamageSystem/S_Damageinfo` 20.0 "NewEnumerator2"))
                (`GameplayStatics.ApplyDamage` _attacktarget 20.0)))
            (:`else`)))))))

(event `/Game/Enemies/AI/BPI_EnemyAI_Base.EquipWeapon`
  (bind _returnvalue (`|SpawnActorFromClass` "/Game/Weapons_Free/Meshes/Actors/AC_pistol_001.AC_pistol_001_C" (`self.GetTransform`) "Undefined" "MultiplyWithRoot" null null))
  (bind _output_get (set `self.PistolActor` _returnvalue))
  (`self.K2_AttachToComponent` _output_get (`self.Mesh`) "hand_r_pistol" "SnapToTarget" "SnapToTarget" "SnapToTarget" true))

(fn `UserConstructionScript`
  (`parent.UserConstructionScript`))