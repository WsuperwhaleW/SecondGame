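; Base enemy character that forwards health, healing and damage calls to a damage system component and exposes its patrol route and preset movement speeds.
; On BeginPlay it caches its AI controller, creates a health bar widget and binds a death event.
; The health bar shows while the player character overlaps a sphere.
; Death ragdolls the mesh, stops the AI brain logic and sets the controller's dead state.
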(event `self.ReceiveBeginPlay`
  (bind _asaic_enemy_base (cast `/Game/Enemies/AI/AIC_Enemy_Base` (`AIBlueprintHelperLibrary.GetAIController` self)))
  (set `self.AICEnemyBase` _asaic_enemy_base)
  (bind _returnvalue (`|CreateWidget` "/Game/DamageSystem/W_HealthBar.W_HealthBar_C" null self))
  (`WidgetComponent.SetWidget` (`self.HealthBar`) _returnvalue)
  (add `/Game/DamageSystem/BPC_DamageSystem.OnDeath` (`self.BPC_DamageSystem`) (`|CreateDelegate` :!event `Die`)))

(event `Die`
  (bind _mesh (`self.Mesh`))
  (`PrimitiveComponent.SetSimulatePhysics` _mesh true)
  (`PrimitiveComponent.SetCollisionEnabled` _mesh "QueryAndPhysics")
  (`BrainComponent.StopLogic` (`AIController.BrainComponent` (`self.AICEnemyBase`)) "")
  (`/Game/Enemies/AI/AIC_Enemy_Base.SetStateAsDead` (`self.AICEnemyBase`)))

(event `self.Sphere.OnComponentBeginOverlap`
  (params (OverlappedComponent :type "PrimitiveComponent Object Reference") (OtherActor :type "Actor Object Reference") (OtherComp :type "PrimitiveComponent Object Reference") (OtherBodyIndex :type Integer) (bFromSweep :type Boolean) (SweepResult :type "HitResult Structure (by ref)"))
  (cast `/Game/ThirdPerson/Blueprints/BP_ThirdPersonCharacter` OtherActor)
  (`SceneComponent.SetVisibility` (`self.HealthBar`) true false))

(event `self.Sphere.OnComponentEndOverlap`
  (params (OverlappedComponent :type "PrimitiveComponent Object Reference") (OtherActor :type "Actor Object Reference") (OtherComp :type "PrimitiveComponent Object Reference") (OtherBodyIndex :type Integer))
  (cast `/Game/ThirdPerson/Blueprints/BP_ThirdPersonCharacter` OtherActor)
  (`SceneComponent.SetVisibility` (`self.HealthBar`) false false))

(fn `GetCurrentHealth`
  (returns (Health :type "Float (double-precision)"))
  (return (`/Game/DamageSystem/BPC_DamageSystem.Health` (`self.BPC_DamageSystem`))))

(fn `GetMaxHealth`
  (returns (MaxHealth :type "Float (double-precision)"))
  (return (`/Game/DamageSystem/BPC_DamageSystem.MaxHealth` (`self.BPC_DamageSystem`))))

(fn `GetPatrolRoute`
  (returns (PatrolRoute :type "/Game/Enemies/AI/BP_PatrolRoute Object Reference"))
  (return (`self.PatrolRoute`)))

(fn `Heal`
  (params (Amount :type "Float (double-precision)"))
  (returns (NewHealth :type "Float (double-precision)"))
  (bind _newhealth (`/Game/DamageSystem/BPC_DamageSystem.Heal` (`self.BPC_DamageSystem`) Amount))
  (return _newhealth))

(fn `IsDead`
  (returns (Dead :type Boolean))
  (return (`/Game/DamageSystem/BPC_DamageSystem.IsDead` (`self.BPC_DamageSystem`))))

(fn `SetMovementSpeed`
  (params (Speed :type "/Game/Enemies/AI/Enums/E_MovementSpeed Enum" :default "NewEnumerator0"))
  (returns (SpeedValue :type "Float (double-precision)"))
  (bind _output_get (set `CharacterMovementComponent.MaxWalkSpeed` (select `/Game/Enemies/AI/Enums/E_MovementSpeed` Speed :`NewEnumerator1` 100.0 :`NewEnumerator2` 300.0 :`NewEnumerator3` 500.0 :!type "Float (single-precision)") (`self.CharacterMovement`)))
  (return _output_get))

(fn `TakeDamage`
  (params (DamageInfo :type "/Game/DamageSystem/S_Damageinfo Structure"))
  (returns (WasDamage :type Boolean))
  (bind _wasdamaged (`/Game/DamageSystem/BPC_DamageSystem.TakeDamage` (`self.BPC_DamageSystem`) DamageInfo))
  (return _wasdamaged))

(fn `UserConstructionScript`)