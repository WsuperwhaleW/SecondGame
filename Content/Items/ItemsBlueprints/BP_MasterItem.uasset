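; BP_MasterItem is an item actor that BP_ThirdPersonCharacter can pick up.
; Overlapping its PickUpRadius with that character caches the character and enables player 0 input on the item, so pressing E passes ItemInfo to PickItem and destroys the item.
; End overlap also calls EnableInput rather than disabling it, so E stays active after leaving the radius.
; HandleAttack and the construction script are empty.
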(event `Key|E`
  (params (Key :type "Key Structure"))
  (:`Pressed`
    (`/Game/ThirdPerson/Blueprints/BP_ThirdPersonCharacter.Pick_Item` (`self.As BP Third Person Character`) (`self.ItemInfo`))
    (`self.K2_DestroyActor`)))

(event `self.PickUpRadius.OnComponentBeginOverlap`
  (params (OverlappedComponent :type "PrimitiveComponent Object Reference") (OtherActor :type "Actor Object Reference") (OtherComp :type "PrimitiveComponent Object Reference") (OtherBodyIndex :type Integer) (bFromSweep :type Boolean) (SweepResult :type "HitResult Structure (by ref)"))
  (bind _asbp_third_person_character (cast `/Game/ThirdPerson/Blueprints/BP_ThirdPersonCharacter` OtherActor))
  (set `self.As BP Third Person Character` _asbp_third_person_character)
  (`self.EnableInput` (`GameplayStatics.GetPlayerController` 0)))

(event `self.PickUpRadius.OnComponentEndOverlap`
  (params (OverlappedComponent :type "PrimitiveComponent Object Reference") (OtherActor :type "Actor Object Reference") (OtherComp :type "PrimitiveComponent Object Reference") (OtherBodyIndex :type Integer))
  (`self.EnableInput` (`GameplayStatics.GetPlayerController` 0)))

(event `Handle Attack`)

(fn `UserConstructionScript`)